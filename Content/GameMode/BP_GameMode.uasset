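; Game mode that runs a minutes-and-seconds countdown and continuously spawns BP_Enemy around the player.
; BeginPlay caches the BP_Marko pawn and player controller and starts one-second looping timers for SetCountdown and SpawnOnTimer.
; GetSpawnTransform picks a random screen side and offsets half the viewport size from the deprojected camera position.
; A self-repeating, delayed SpawnEnemy batch event exists but is not triggered in this graph.
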(event `self.ReceiveBeginPlay`
  (`KismetSystemLibrary.K2_SetTimer` null "SetCountdown" 1.0 true)
  (bind _asbp_marko (cast `/Game/Pawns2D/BP_Marko` (`GameplayStatics.GetPlayerPawn` 0)))
  (set `self.Player` _asbp_marko)
  (bind _asbp_player_controller (cast `/Game/Controller/BP_PlayerController` (`GameplayStatics.GetPlayerController` 0)))
  (set `self.PlayerController` _asbp_player_controller)
  (`KismetSystemLibrary.K2_SetTimer` null "SpawnOnTimer" 1.0 true))

(event `self.ReceiveTick`
  (params (DeltaSeconds :type "Float (single-precision)")))

(event `SpawnEnemy`
  (params (Class :type "Actor Class Reference") (SpawnTransform :type "Transform Structure") (NumberOfEnemys :type Integer))
  ;[1 1 1] SpawnEnemys
  (for _ (range (+ NumberOfEnemys 1))
    (`|SpawnActorFromClass` Class SpawnTransform "AdjustIfPossibleButAlwaysSpawn" "OverrideRootScale" null null))
  (`KismetSystemLibrary.Delay` (`self.SpawnDelay`))
  (bind (_enemyx _enemyy) (`self.GetSpawnTransform`))
  (`self.SpawnEnemy` "/Game/Pawns2D/Enemys/BP_Enemy.BP_Enemy_C" (`KismetMathLibrary.MakeTransform` (`KismetMathLibrary.MakeVector` _enemyx _enemyy 20.0)) (`self.Number Of Enemys`)))

(fn `GetSpawnTransform`
  (returns (EnemyX :type "Float (double-precision)") (EnemyY :type "Float (double-precision)"))
  (locals (ScreenSides :type Integer) (X :type "Float (double-precision)") (Y :type "Float (double-precision)"))
  (bind _returnvalue_x (`KismetMathLibrary.BreakVector2D` (`WidgetLayoutLibrary.GetViewportSize`)))
  (bind (_returnvalue_x_2 _returnvalue_y) (`KismetMathLibrary.BreakVector2D` (`WidgetLayoutLibrary.GetViewportSize`)))
  (bind _returnvalue_x_3 (`KismetMathLibrary.BreakVector2D` (`WidgetLayoutLibrary.GetViewportSize`)))
  (bind (_returnvalue_x_4 _returnvalue_y_2) (`KismetMathLibrary.BreakVector2D` (`WidgetLayoutLibrary.GetViewportSize`)))
  (bind (_returnvalue_x_5 _returnvalue_y_3) (`KismetMathLibrary.BreakVector2D` (`WidgetLayoutLibrary.GetViewportSize`)))
  (bind (_returnvalue_x_6 _returnvalue_y_4) (`KismetMathLibrary.BreakVector2D` (`WidgetLayoutLibrary.GetViewportSize`)))
  (bind _returnvalue_x_7 (`KismetMathLibrary.BreakVector2D` (`WidgetLayoutLibrary.GetViewportSize`)))
  (bind _returnvalue_x_8 (`KismetMathLibrary.BreakVector2D` (`WidgetLayoutLibrary.GetViewportSize`)))
  (bind _returnvalue (/ _returnvalue_y_2 2.0))
  (bind _returnvalue_2 (/ _returnvalue_y_3 2.0))
  (bind _returnvalue_3 (/ _returnvalue_x_7 2.0))
  (bind _returnvalue_4 (/ _returnvalue_x_8 2.0))
  (bind _worldposition (`GameplayStatics.DeprojectScreenToWorld` (`self.PlayerController`) (`KismetMathLibrary.Conv_VectorToVector2D` (`SceneComponent.K2_GetComponentLocation` (`/Game/Pawns2D/BP_Marko.Camera` (`self.Player`))))))
  (bind _worldposition_2 (`GameplayStatics.DeprojectScreenToWorld` (`self.PlayerController`) (`KismetMathLibrary.Conv_VectorToVector2D` (`SceneComponent.K2_GetComponentLocation` (`/Game/Pawns2D/BP_Marko.Camera` (`self.Player`))))))
  (bind _worldposition_3 (`GameplayStatics.DeprojectScreenToWorld` (`self.PlayerController`) (`KismetMathLibrary.Conv_VectorToVector2D` (`SceneComponent.K2_GetComponentLocation` (`/Game/Pawns2D/BP_Marko.Camera` (`self.Player`))))))
  (bind _worldposition_4 (`GameplayStatics.DeprojectScreenToWorld` (`self.PlayerController`) (`KismetMathLibrary.Conv_VectorToVector2D` (`SceneComponent.K2_GetComponentLocation` (`/Game/Pawns2D/BP_Marko.Camera` (`self.Player`))))))
  (bind _output_get (set `local.ScreenSides` (`KismetMathLibrary.RandomIntegerInRange` 0 3)))
  (switch `int` _output_get
    (:`0`
      (return (- (- (.x _worldposition) (/ _returnvalue_x 2.0)) 1.0) (+ (.y _worldposition) (`KismetMathLibrary.RandomFloatInRange` (* _returnvalue -1.0) _returnvalue))))
    (:`1`
      (return (+ (+ (/ _returnvalue_x_3 2.0) (.x _worldposition_4)) 1.0) (+ (.y _worldposition_4) (`KismetMathLibrary.RandomFloatInRange` (* _returnvalue_2 -1.0) _returnvalue_2))))
    (:`2`
      (return (+ (.x _worldposition_3) (`KismetMathLibrary.RandomFloatInRange` (* _returnvalue_3 -1.0) _returnvalue_3)) (- (- (.y _worldposition_3) (/ _returnvalue_y 2.0)) 1.0)))
    (:`3`
      (return (+ (.x _worldposition_2) (`KismetMathLibrary.RandomFloatInRange` (* _returnvalue_4 -1.0) _returnvalue_4)) (+ (+ (.y _worldposition_2) (/ _returnvalue_y_4 2.0)) 1.0)))))

(fn `SetCountdown`
  (set `self.Seconds` (- (`self.Seconds`) 1))
  (if (== (`self.Seconds`) 0)
    (set `self.Minutes` (- (`self.Minutes`) 1))
    (set `self.Seconds` 60)))

(fn `SpawnOnTimer`
  (bind (_enemyx _enemyy) (`self.GetSpawnTransform`))
  (`|SpawnActorFromClass` "/Game/Pawns2D/Enemys/BP_Enemy.BP_Enemy_C" (`KismetMathLibrary.MakeTransform` (`KismetMathLibrary.MakeVector` _enemyx _enemyy)) "AdjustIfPossibleButAlwaysSpawn" "OverrideRootScale" null null))

(fn `UserConstructionScript`)