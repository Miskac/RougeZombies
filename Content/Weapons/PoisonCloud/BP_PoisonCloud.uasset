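; BP_PoisonCloud is a short-lived weapon area-of-effect actor that deals a single burst of damage to enemies.
; On BeginPlay it sets Damage from the player's poison cloud damage and damage multiplier, then gives itself a one-second lifespan.
; After a brief delay it applies that damage once to every BP_Enemy overlapping its HitBox, crediting the player as instigator and causer.
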(event `self.ReceiveBeginPlay`
  (bind _player (`self.Player`))
  (`parent.ReceiveBeginPlay`)
  (`self.InicializeStats`)
  (`self.SetLifeSpan` 1.0)
  (`KismetSystemLibrary.Delay` 0.2)
  (for _array_element (`PrimitiveComponent.GetOverlappingActors` (`self.HitBox`) "/Game/Pawns2D/Enemys/BP_Enemy.BP_Enemy_C")
    (`GameplayStatics.ApplyDamage` _array_element (`self.Damage`) (`Pawn.GetController` _player) _player "/Script/Engine.DamageType")))

(fn `InicializeStats`
  (bind _player (`self.Player`))
  (`parent.InicializeStats`)
  (set `self.Damage` (* (`/Game/Pawns2D/BP_Marko.PoisonCloudDamage` _player) (`/Game/Pawns2D/BP_Marko.DamageMultiplayer` _player))))

(fn `UserConstructionScript`
  (`parent.UserConstructionScript`))