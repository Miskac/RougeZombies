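; BP_Weapon is a weapon actor that provides enemy targeting, with FireWeapon and GetClosestEnemyToWeapon left as empty stubs.
; On BeginPlay it caches the BP_GameMode and the BP_Marko player.
; GetClosestEnemy linearly scans "Homing"-tagged BP_Enemy actors for the one horizontally nearest the player, without guarding against an empty list.
; Tick is empty, and a debug line to that enemy is disconnected.
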(event `self.ReceiveBeginPlay`
  (bind _asbp_game_mode (cast `/Game/GameMode/BP_GameMode` (`GameplayStatics.GetGameMode`)))
  (set `self.GameMode` _asbp_game_mode)
  (bind _asbp_marko (cast `/Game/Pawns2D/BP_Marko` (`GameplayStatics.GetPlayerPawn` 0)))
  (set `self.Player` _asbp_marko))

(event `self.ReceiveTick`
  (params (DeltaSeconds :type "Float (single-precision)")))

(fn `FireWeapon`)

(fn `GetClosestEnemy`
  (returns (ClosesEnemy :type "/Game/Pawns2D/Enemys/BP_Enemy Object Reference"))
  (locals (CurrentClosesEnemy :type "/Game/Pawns2D/Enemys/BP_Enemy Object Reference"))
  (bind _outactors (`GameplayStatics.GetAllActorsOfClassWithTag` "/Game/Pawns2D/Enemys/BP_Enemy.BP_Enemy_C" "Homing"))
  (set `local.CurrentClosesEnemy` (`|GetArrayItem` _outactors))
  (for (_array_element _array_index) _outactors
    (if (!= _array_index 0)
      (if (<= (`self.GetHorizontalDistanceTo` _array_element (`self.Player`)) (`self.GetHorizontalDistanceTo` (`local.CurrentClosesEnemy`) (`self.Player`)))
        (set `local.CurrentClosesEnemy` _array_element))))
  (return (`local.CurrentClosesEnemy`)))

(fn `GetClosestEnemyToWeapon`)

(fn `UserConstructionScript`)