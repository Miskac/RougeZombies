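; BP_FanOfKnifes is a short-lived knife weapon actor that damages the first BP_Enemy it overlaps, then destroys itself.
; InicializeStats scales damage from the Player's knife stat and multiplier.
; FireWeapon and FireMore spawn a ring of copies of this same class by stepping yaw in fixed increments.
; The Box overlap handler confirms enemies by searching all BP_Enemy actors, then applies point damage credited to the Player.
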(event `self.ReceiveBeginPlay`
  (`parent.ReceiveBeginPlay`)
  (`self.InicializeStats`)
  (add `PrimitiveComponent.OnComponentBeginOverlap` (`self.Box`) (delegate `OnComponentBeginOverlap_Event_0`))
  (`self.SetLifeSpan` 0.5))

(event `OnComponentBeginOverlap_Event_0`
  (params (OverlappedComponent :type "PrimitiveComponent Object Reference") (OtherActor :type "Actor Object Reference") (OtherComp :type "PrimitiveComponent Object Reference") (OtherBodyIndex :type Integer) (bFromSweep :type Boolean) (SweepResult :type "HitResult Structure (by ref)"))
  (bind _player (`self.Player`))
  (bind _outactors (`GameplayStatics.GetAllActorsOfClass` "/Game/Pawns2D/Enemys/BP_Enemy.BP_Enemy_C"))
  (for _array_element _outactors
    (`/Engine/EditorBlueprintResources/StandardMacros.IsValid` _array_element
      (:`Is Valid`
        (if (== _array_element OtherActor)
          (`GameplayStatics.ApplyPointDamage` OtherActor (`self.Damage`) (- (`self.K2_GetActorLocation` OtherActor) (`self.K2_GetActorLocation`)) SweepResult (`Pawn.GetController` _player) _player "/Script/Engine.DamageType")
          (`self.K2_DestroyActor`)
          (break))))))

(fn `FireMore`
  (bind _returnvalue (`self.GetTransform`))
  (for _ (range 11)
    (set `self.RotationZ` (+ (`self.RotationZ`) 30.0))
    (`|SpawnActorFromClass` "BP_FanOfKnifes_C" (`KismetMathLibrary.MakeTransform` (.location _returnvalue) (`KismetMathLibrary.MakeRotator` (.roll (.rotation _returnvalue)) (.pitch (.rotation _returnvalue)) (`self.RotationZ`)) (.scale _returnvalue)) "AdjustIfPossibleButAlwaysSpawn" "OverrideRootScale" null (`self.Player`)))
  (set `self.RotationZ` 0.0)
  (return))

(fn `FireWeapon`
  (bind _returnvalue (`self.GetTransform`))
  (`parent.FireWeapon`)
  (for _ (range 11)
    (set `self.RotationZ` (+ (`self.RotationZ`) 30.0))
    (`|SpawnActorFromClass` "BP_FanOfKnifes_C" (`KismetMathLibrary.MakeTransform` (.location _returnvalue) (`KismetMathLibrary.MakeRotator` (.roll (.rotation _returnvalue)) (.pitch (.rotation _returnvalue)) (`self.RotationZ`)) (.scale _returnvalue)) "AdjustIfPossibleButAlwaysSpawn" "OverrideRootScale" null (`self.Player`)))
  (set `self.RotationZ` 0.0)
  (return))

(fn `InicializeStats`
  (bind _player (`self.Player`))
  (`parent.InicializeStats`)
  (set `self.Damage` (* (`/Game/Pawns2D/BP_Marko.FanOfKnifesDamage` _player) (`/Game/Pawns2D/BP_Marko.DamageMultiplayer` _player))))

(fn `UserConstructionScript`
  (`parent.UserConstructionScript`))