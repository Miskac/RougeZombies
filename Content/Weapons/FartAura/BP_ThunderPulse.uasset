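; BP_ThunderPulse is an aura weapon that attaches to the player and periodically deals full radial damage around itself.
; On BeginPlay it sets damage and mana cost, then starts a looping DamagePulse timer using the HitBox radius and the player's damage amplifier.
; Tick destroys the actor when more than one pulse exists.
; An armor-reduced overlap damage handler remains, but its binding never runs.
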(event `OnComponentBeginOverlap_Event_0`
  (params (OverlappedComponent :type "PrimitiveComponent Object Reference") (OtherActor :type "Actor Object Reference") (OtherComp :type "PrimitiveComponent Object Reference") (OtherBodyIndex :type Integer) (bFromSweep :type Boolean) (SweepResult :type "HitResult Structure (by ref)"))
  (bind _player (`self.Player`))
  ;[1 1 1] DealDamage
  (bind _outactors (`GameplayStatics.GetAllActorsOfClass` "/Game/Pawns2D/Enemys/BP_Enemy.BP_Enemy_C"))
  (for _array_element _outactors
    (`/Engine/EditorBlueprintResources/StandardMacros.IsValid` _array_element
      (:`Is Valid`
        (if (== (`/Game/Pawns2D/Enemys/BP_Enemy.HitBox` _array_element) OtherComp)
          (`GameplayStatics.ApplyDamage` _array_element (- (* (`self.Damage`) (`/Game/Pawns2D/BP_Marko.BaseDamageAmplifier` _player)) (`/Game/Pawns2D/Enemys/BP_Enemy.Armor` _array_element)) (`Pawn.GetController` _player) _player "/Script/Engine.DamageType"))))))

(event `self.ReceiveBeginPlay`
  (bind _player (`self.Player`))
  (`parent.ReceiveBeginPlay`)
  (set `self.Damage` 5.0)
  (set `self.ManaCost` 1.0)
  (`/Engine/EditorBlueprintResources/StandardMacros.IsValid` _player
    (:`Is Valid`
      (`self.K2_AttachToActor` _player "None" "SnapToTarget" "SnapToTarget" "KeepRelative")
      (`KismetSystemLibrary.K2_SetTimer` null "DamagePulse" 1.0 true))))

(event `self.ReceiveTick`
  (params (DeltaSeconds :type "Float (single-precision)"))
  (`parent.ReceiveTick` DeltaSeconds)
  (bind _outactors (`GameplayStatics.GetAllActorsOfClass` "BP_ThunderPulse_C"))
  (if (> (`KismetArrayLibrary.Array_Length` _outactors) 1)
    (`self.K2_DestroyActor`)))

(fn `DamagePulse`
  (bind _player (`self.Player`))
  (`GameplayStatics.ApplyRadialDamage` (* (`self.Damage`) (`/Game/Pawns2D/BP_Marko.BaseDamageAmplifier` _player)) (`self.K2_GetActorLocation`) (`SphereComponent.SphereRadius` (`self.HitBox`)) "/Script/Engine.DamageType" (`|MakeArray` _player :!type "Actor Object Reference") _player (`Pawn.GetController` _player) true))

(fn `UserConstructionScript`
  (`parent.UserConstructionScript`))