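; Chain lightning projectile weapon that homes in on enemies and bounces between them, with damage, mana cost and bounce limit taken from Player stats.
; FireWeapon aims the homing ProjectileMovement at the closest enemy.
; HitBox overlaps deal point damage minus Armor, then retarget via the hit enemy's GetClosestEnemyToYou until MaxBounces destroys it, with a lifespan as backstop.
; GetClosestEnemyToLastEnemy searches "Homing"-tagged enemies but is not called here.
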(event `self.ReceiveBeginPlay`
  (`parent.ReceiveBeginPlay`)
  (`self.InicializeStats`)
  (add `PrimitiveComponent.OnComponentBeginOverlap` (`self.HitBox`) (delegate `OnComponentBeginOverlap_Event_0`))
  (`self.SetLifeSpan` 5.0))

(event `OnComponentBeginOverlap_Event_0`
  (params (OverlappedComponent :type "PrimitiveComponent Object Reference") (OtherActor :type "Actor Object Reference") (OtherComp :type "PrimitiveComponent Object Reference") (OtherBodyIndex :type Integer) (bFromSweep :type Boolean) (SweepResult :type "HitResult Structure (by ref)"))
  (bind _player (`self.Player`))
  (bind _outactors (`GameplayStatics.GetAllActorsOfClass` "/Game/Pawns2D/Enemys/BP_Enemy.BP_Enemy_C"))
  (for _array_element _outactors
    (`/Engine/EditorBlueprintResources/StandardMacros.IsValid` _array_element
      (:`Is Valid`
        (if (== (`/Game/Pawns2D/Enemys/BP_Enemy.HitBox` _array_element) OtherComp)
          (`/Engine/EditorBlueprintResources/StandardMacros.IncrementInt` (`self.Bounces`)
            (:`  `
              (`GameplayStatics.ApplyPointDamage` OtherActor (- (`self.Damage`) (`/Game/Pawns2D/Enemys/BP_Enemy.Armor` _array_element)) (- (`self.K2_GetActorLocation` _array_element) (`self.K2_GetActorLocation`)) SweepResult (`Pawn.GetController` _player) _player "/Script/Engine.DamageType")
              (if (< (`self.Bounces`) (`self.MaxBounces`))
                (bind _asbp_enemy (cast `/Game/Pawns2D/Enemys/BP_Enemy` OtherActor))
                (bind _closest (`/Game/Pawns2D/Enemys/BP_Enemy.GetClosestEnemyToYou` _asbp_enemy))
                (set `ProjectileMovementComponent.HomingTargetComponent` (`self.GetComponentByClass` _closest "/Script/Engine.SceneComponent") (`self.ProjectileMovement`))
                (else
                  (`self.K2_DestroyActor`))))))))))

(event `self.ReceiveTick`
  (params (DeltaSeconds :type "Float (single-precision)"))
  (`parent.ReceiveTick` DeltaSeconds))

(fn `FireWeapon`
  (`parent.FireWeapon`)
  (bind _closesenemy (`self.GetClosestEnemy`))
  (set `ProjectileMovementComponent.HomingTargetComponent` (`self.GetComponentByClass` _closesenemy "/Script/Engine.SceneComponent") (`self.ProjectileMovement`)))

(fn `GetClosestEnemyToLastEnemy`
  (params (LastHitEnemy :type "/Game/Pawns2D/Enemys/BP_Enemy Object Reference"))
  (returns (ClosestEnemy :type "/Game/Pawns2D/Enemys/BP_Enemy Object Reference"))
  (locals (CurrentClosestEnemy :type "/Game/Pawns2D/Enemys/BP_Enemy Object Reference") (LastEnemyHit :type "/Game/Pawns2D/Enemys/BP_Enemy Object Reference"))
  (bind _lastenemyhit (`local.LastEnemyHit`))
  (set `local.LastEnemyHit` LastHitEnemy)
  (bind _outactors (`GameplayStatics.GetAllActorsOfClassWithTag` "/Game/Pawns2D/Enemys/BP_Enemy.BP_Enemy_C" "Homing"))
  (set `local.CurrentClosestEnemy` (`|GetArrayItem` _outactors))
  (for (_array_element _array_index) _outactors
    (if (!= _array_index 0)
      (if (<= (`self.GetHorizontalDistanceTo` _array_element _lastenemyhit) (`self.GetHorizontalDistanceTo` (`local.CurrentClosestEnemy`) _lastenemyhit))
        (set `local.CurrentClosestEnemy` _array_element))))
  (return (`local.CurrentClosestEnemy`)))

(fn `InicializeStats`
  (bind _player (`self.Player`))
  (`parent.InicializeStats`)
  (set `self.Damage` (* (`/Game/Pawns2D/BP_Marko.ChainLightningDamage` _player) (`/Game/Pawns2D/BP_Marko.BaseDamageAmplifier` _player)))
  (set `self.ManaCost` (`/Game/Pawns2D/BP_Marko.ChainLightningManaCost` _player))
  (set `self.MaxBounces` (`/Game/Pawns2D/BP_Marko.ChainLightningBounces` _player)))

(fn `UserConstructionScript`
  (`parent.UserConstructionScript`))