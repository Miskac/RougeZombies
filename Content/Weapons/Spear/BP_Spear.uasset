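; BP_Spear is a thrown spear weapon that flies at the player's spear target, damages an enemy and returns to the player.
; It reads damage and target from the player, launches horizontally through ProjectileMovement, and applies point damage when HitBox overlaps a BP_Enemy.
; After a hit, Tick steers it back toward the player at max speed, destroying it on arrival.
; A five-second lifespan also limits the spear.
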(event `self.ReceiveBeginPlay`
  (bind _projectilemovement (`self.ProjectileMovement`))
  (`parent.ReceiveBeginPlay`)
  (`self.InicializeStats`)
  (add `PrimitiveComponent.OnComponentBeginOverlap` (`self.HitBox`) (delegate `OnComponentBeginOverlap_Event_0`))
  (set `MovementComponent.Velocity` (* (`KismetMathLibrary.Vector_Normal2D` (- (`self.K2_GetActorLocation` (`self.Target`)) (`self.K2_GetActorLocation`))) (`ProjectileMovementComponent.InitialSpeed` _projectilemovement)) _projectilemovement)
  (`self.SetLifeSpan` 5.0))

(event `OnComponentBeginOverlap_Event_0`
  (params (OverlappedComponent :type "PrimitiveComponent Object Reference") (OtherActor :type "Actor Object Reference") (OtherComp :type "PrimitiveComponent Object Reference") (OtherBodyIndex :type Integer) (bFromSweep :type Boolean) (SweepResult :type "HitResult Structure (by ref)"))
  (bind _player (`self.Player`))
  (bind _outactors (`GameplayStatics.GetAllActorsOfClass` "/Game/Pawns2D/Enemys/BP_Enemy.BP_Enemy_C"))
  (for _array_element _outactors
    (`/Engine/EditorBlueprintResources/StandardMacros.IsValid` _array_element
      (:`Is Valid`
        (if (== _array_element OtherActor)
          (`GameplayStatics.ApplyPointDamage` OtherActor (`self.Damage`) (- (`self.K2_GetActorLocation` OtherActor) (`self.K2_GetActorLocation`)) SweepResult (`Pawn.GetController` _player) _player "/Script/Engine.DamageType")
          (set `self.Hit` true)
          (break))))))

(event `self.ReceiveTick`
  (params (DeltaSeconds :type "Float (single-precision)"))
  (bind _projectilemovement (`self.ProjectileMovement`))
  (`parent.ReceiveTick` DeltaSeconds)
  (if (`self.Hit`)
    (set `ProjectileMovementComponent.bRotationFollowsVelocity` false (`self.ProjectileMovement`))
    (bind _output_get (set `MovementComponent.Velocity` (* (`KismetMathLibrary.Vector_Normal2D` (- (`self.K2_GetActorLocation` (`self.Player`)) (`self.K2_GetActorLocation`))) (`ProjectileMovementComponent.MaxSpeed` _projectilemovement)) _projectilemovement))
    (`SceneComponent.K2_SetRelativeRotation` (`self.DefaultSceneRoot`) (`KismetMathLibrary.Conv_VectorToRotator` (* _output_get (`self.Direction`))) false false)
    (if (<= (`self.GetHorizontalDistanceTo` (`self.Player`) self) 10.0)
      (`self.K2_DestroyActor`))))

(fn `FireWeapon`
  (`parent.FireWeapon`))

(fn `InicializeStats`
  (bind _player (`self.Player`))
  (`parent.InicializeStats`)
  (set `self.Damage` (* (`/Game/Pawns2D/BP_Marko.SpearDamage` _player) (`/Game/Pawns2D/BP_Marko.DamageMultiplayer` _player)))
  (set `self.Target` (`/Game/Pawns2D/BP_Marko.SpearsTarget` _player))
  (set `self.Hit` false))

(fn `UserConstructionScript`
  (`parent.UserConstructionScript`))