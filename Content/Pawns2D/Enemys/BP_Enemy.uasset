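; 2D enemy pawn that chases the player, attacks on contact and drops experience on death.
; Tick runs AI MoveTo toward the GameMode's player and switches idle/walk flipbooks.
; HitBox overlap with BP_Marko's HitBox starts a delay-looped attack, reduced by armor, until overlap end clears the target.
; Taking damage lowers health and staggers movement; death plays a flipbook, spawns BP_EXP and destroys the actor after a delay.
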(event `OnComponentEndOverlap_Event_0`
  (params (OverlappedComponent :type "PrimitiveComponent Object Reference") (OtherActor :type "Actor Object Reference") (OtherComp :type "PrimitiveComponent Object Reference") (OtherBodyIndex :type Integer))
  ;[1 1 1] Stop Attacking
  (bind _asbp_marko (cast `/Game/Pawns2D/BP_Marko` OtherActor))
  (if (== (`/Game/Pawns2D/BP_Marko.HitBox` _asbp_marko) OtherComp)
    (set `self.bAttacking` false)
    (`PaperFlipbookComponent.SetFlipbook` (`self.Sprite`) (`self.IdleSprite`))
    (set `self.PlayerCharacter` null)))

(event `self.ReceiveBeginPlay`
  (bind _hitbox (`self.HitBox`))
  ;[1 1 1] BeginPlay
  (bind _asenemy_hpbar (cast `/Game/Pawns2D/Enemys/EnemyHPBar` (`WidgetComponent.GetUserWidgetObject` (`self.HPBar`))))
  (set `/Game/Pawns2D/Enemys/EnemyHPBar.EnemyPawn` self _asenemy_hpbar)
  (`SphereComponent.SetSphereRadius` (`self.HitBox`) (`self.HitBoxRadius`) true)
  (add `PrimitiveComponent.OnComponentBeginOverlap` _hitbox (delegate `OnComponentBeginOverlap_Event_0`))
  (add `PrimitiveComponent.OnComponentEndOverlap` _hitbox (delegate `OnComponentEndOverlap_Event_0`))
  (bind _asaicontroller (cast `AIController` (`self.GetController`)))
  (set `self.AIController` _asaicontroller)
  (bind _asbp_game_mode (cast `/Game/GameMode/BP_GameMode` (`GameplayStatics.GetGameMode`)))
  (set `self.GameMode` _asbp_game_mode)
  (set `self.Player` (`/Game/GameMode/BP_GameMode.Player` _asbp_game_mode)))

(event `OnComponentBeginOverlap_Event_0`
  (params (OverlappedComponent :type "PrimitiveComponent Object Reference") (OtherActor :type "Actor Object Reference") (OtherComp :type "PrimitiveComponent Object Reference") (OtherBodyIndex :type Integer) (bFromSweep :type Boolean) (SweepResult :type "HitResult Structure (by ref)"))
  ;[1 1 1] Attack
  (bind _asbp_marko (cast `/Game/Pawns2D/BP_Marko` OtherActor))
  (set `self.PlayerCharacter` _asbp_marko)
  (if (== (`/Game/Pawns2D/BP_Marko.HitBox` _asbp_marko) OtherComp)
    (if (not (`self.bIsDead`))
      (set `self.bAttacking` true)
      (`PaperFlipbookComponent.SetFlipbook` (`self.Sprite`) (`self.AttackSprite`))
      (`GameplayStatics.ApplyDamage` _asbp_marko (- (`self.BaseDamage`) (`/Game/Pawns2D/BP_Marko.Armor` (`self.PlayerCharacter`))) null self "/Script/Engine.DamageType" :!label _label)
      (`KismetSystemLibrary.Delay` (`self.AttackSpeed`))
      (`/Engine/EditorBlueprintResources/StandardMacros.IsValid` (`self.PlayerCharacter`)
        (:`Is Valid`
          (goto _label))))))

(event `self.ReceiveTick`
  (params (DeltaSeconds :type "Float (single-precision)"))
  (bind _player (`self.Player`))
  (bind _asbp_game_mode (cast `/Game/GameMode/BP_GameMode` (`GameplayStatics.GetGameMode`)))
  (set `self.GameMode` _asbp_game_mode)
  (set `self.Player` (`/Game/GameMode/BP_GameMode.Player` _asbp_game_mode))
  (if (`self.bTakenDamage`)
    (`KismetSystemLibrary.Delay` (`self.StaggerDuration`))
    (set `self.bTakenDamage` false)
    (elif (not (`self.bIsDead`))
      (`|AIMoveTo` self (`self.K2_GetActorLocation` _player) _player 1.0
        (:`then`
          (if (`self.bAttacking`)
            _
            (elif (`self.bIsDead`)
              _
              (elif (== (`self.GetVelocity`) (0.0 0.0 0.0))
                (`PaperFlipbookComponent.SetFlipbook` (`self.Sprite`) (`self.IdleSprite`))
                (else
                  (`PaperFlipbookComponent.SetFlipbook` (`self.Sprite`) (`self.WalkSprite`)))))))))))

(event `self.ReceiveAnyDamage`
  (params (Damage :type "Float (single-precision)") (DamageType :type "DamageType Object Reference") (InstigatedBy :type "Controller Object Reference") (DamageCauser :type "Actor Object Reference"))
  (set `self.bTakenDamage` true)
  (`MovementComponent.StopMovementImmediately` (`self.CharacterMovement`))
  (if (<= (- (`self.Health`) Damage) 0.0)
    (set `self.Health` 0.0)
    (else
      (set `self.Health` (- (`self.Health`) Damage))))
  (if (<= (`self.Health`) 0.0)
    ;[1 1 1] Death
    (`Controller.StopMovement` (`self.AIController`))
    (set `self.bIsDead` true)
    (`PaperFlipbookComponent.SetFlipbook` (`self.Sprite`) (`self.DeathSprite`))
    (bind _returnvalue (`|SpawnActorFromClass` "/Game/Pawns2D/Exp/BP_EXP.BP_EXP_C" (`self.GetTransform`) "AdjustIfPossibleButAlwaysSpawn" "OverrideRootScale" null self))
    (set `/Game/Pawns2D/Exp/BP_EXP.ExpAmount` (`self.ExpDropped`) _returnvalue)
    (`KismetSystemLibrary.Delay` 1.0)
    (`self.K2_DestroyActor`)))

(fn `UserConstructionScript`)