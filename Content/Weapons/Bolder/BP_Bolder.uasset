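; BP_Bolder is a boulder projectile weapon that damages BP_Enemy actors and pierces a limited number of them.
; On spawn it takes damage and pierce from Player stats, picks random X speed signed by player rotation, and sets a short lifespan.
; Tick raises Y velocity by a fixed, frame-rate-dependent step, curving its path.
; HitBox overlaps apply point damage, destroying the boulder on the overlap after its pierce limit.
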(event `self.ReceiveBeginPlay`
  (`parent.ReceiveBeginPlay`)
  (`self.InicializeStats`)
  (if (>= (`/Game/Pawns2D/BP_Marko.Rotation` (`self.Player`)) 0.0)
    (set `self.RandX` (`KismetMathLibrary.RandomFloatInRange` 50.0 200.0))
    (else
      (set `self.RandX` (`KismetMathLibrary.RandomFloatInRange` -50.0 -200.0))))
  (`self.SetLifeSpan` 4.0)
  (add `PrimitiveComponent.OnComponentBeginOverlap` (`self.HitBox`) (delegate `OnComponentBeginOverlap_Event_0`)))

(event `OnComponentBeginOverlap_Event_0`
  (params (OverlappedComponent :type "PrimitiveComponent Object Reference") (OtherActor :type "Actor Object Reference") (OtherComp :type "PrimitiveComponent Object Reference") (OtherBodyIndex :type Integer) (bFromSweep :type Boolean) (SweepResult :type "HitResult Structure (by ref)"))
  (bind _player (`self.Player`))
  (bind _outactors (`GameplayStatics.GetAllActorsOfClass` "/Game/Pawns2D/Enemys/BP_Enemy.BP_Enemy_C"))
  (for _array_element _outactors
    (`/Engine/EditorBlueprintResources/StandardMacros.IsValid` _array_element
      (:`Is Valid`
        (if (== _array_element OtherActor)
          (if (>= (`self.Pierce`) (`self.MaxPierce`))
            (`self.K2_DestroyActor`)
            (else
              (`GameplayStatics.ApplyPointDamage` OtherActor (`self.Damage`) (- (`self.K2_GetActorLocation` OtherActor) (`self.K2_GetActorLocation`)) SweepResult (`Pawn.GetController` _player) _player "/Script/Engine.DamageType")
              (`/Engine/EditorBlueprintResources/StandardMacros.IncrementInt` (`self.Pierce`)
                (:`  `
                  (break))))))))))

(event `self.ReceiveTick`
  (params (DeltaSeconds :type "Float (single-precision)"))
  (`parent.ReceiveTick` DeltaSeconds)
  (set `self.DeltaTime` DeltaSeconds)
  (bind _output_get (set `self.SlowingSpeed` (+ (`self.SlowingSpeed`) 4.0)))
  (set `MovementComponent.Velocity` (`KismetMathLibrary.MakeVector` (`self.RandX`) _output_get) (`self.ProjectileMovement`)))

(fn `InicializeStats`
  (bind _player (`self.Player`))
  (`parent.InicializeStats`)
  (set `self.Damage` (* (`/Game/Pawns2D/BP_Marko.BolderDamage` _player) (`/Game/Pawns2D/BP_Marko.DamageMultiplayer` _player)))
  (set `self.MaxPierce` (`/Game/Pawns2D/BP_Marko.BolerPierce` _player)))

(fn `UserConstructionScript`
  (`parent.UserConstructionScript`))