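; Player character Marko for a 2D flipbook auto-attack game, with movement, melee click attack, invulnerable dodge, armor-reduced damage and pause toggle.
; Shortly after BeginPlay, the Weapons array starts looping timers spawning mana-costing sword, magma fist, chakram and chain lightning, while shields and fart aura spawn once.
; Timers regenerate health and mana.
; Tick swaps idle/moving flipbooks and triggers level-up on full Exp, pausing the game for an upgrade menu.
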(event `FiringShield`
  (bind _outactors (`GameplayStatics.GetAllActorsOfClass` "/Game/Weapons/Shield/BP_Shield.BP_Shield_C"))
  (for _array_element _outactors
    (`self.K2_DestroyActor` _array_element))
  (for _index (range 1 (+ (`self.NumberOfScytheProjectiles`) 1))
    (if (== _index 1)
      (bind _returnvalue (`|SpawnActorFromClass` "/Game/Weapons/Shield/BP_Shield.BP_Shield_C" (`self.GetTransform`) "AdjustIfPossibleButAlwaysSpawn" "OverrideRootScale" self self))
      (set `/Game/Weapons/Shield/BP_Shield.Dimentions` (70.0 0.0 0.0) _returnvalue)
      (elif (== _index 2)
        (bind _returnvalue_2 (`|SpawnActorFromClass` "/Game/Weapons/Shield/BP_Shield.BP_Shield_C" (`self.GetTransform`) "AdjustIfPossibleButAlwaysSpawn" "OverrideRootScale" null self))
        (set `/Game/Weapons/Shield/BP_Shield.Dimentions` (-70.0 0.0 0.0) _returnvalue_2)
        (elif (== _index 3)
          (bind _returnvalue_3 (`|SpawnActorFromClass` "/Game/Weapons/Shield/BP_Shield.BP_Shield_C" (`self.GetTransform`) "AdjustIfPossibleButAlwaysSpawn" "OverrideRootScale" null self))
          (set `/Game/Weapons/Shield/BP_Shield.Dimentions` (0.0 -70.0 0.0) _returnvalue_3)
          (elif (== _index 4)
            (bind _returnvalue_4 (`|SpawnActorFromClass` "/Game/Weapons/Shield/BP_Shield.BP_Shield_C" (`self.GetTransform`) "AdjustIfPossibleButAlwaysSpawn" "OverrideRootScale" null self))
            (set `/Game/Weapons/Shield/BP_Shield.Dimentions` (0.0 70.0 0.0) _returnvalue_4)))))))

(event `self.ReceiveBeginPlay`
  ;[1 1 1] BeginPlay
  (bind _asbp_player_controller (cast `/Game/Controller/BP_PlayerController` (`self.GetController`)))
  (set `self.PlayerControlelr` _asbp_player_controller)
  (set `self.Health` (`KismetMathLibrary.FClamp` (`self.Health`) 0.0 (`self.MaxHealth`)))
  (set `self.Mana` (`KismetMathLibrary.FClamp` (`self.Mana`) 0.0 (`self.MaxMana`)))
  (set `self.Exp` (`KismetMathLibrary.FClamp` (`self.Exp`) 0.0 (`self.MaxExp`)))
  (`KismetSystemLibrary.K2_SetTimer` null "HealthRegeneration" 1.0 true)
  (`KismetSystemLibrary.K2_SetTimer` null "ManaRegeneration" 1.0 true)
  (`KismetSystemLibrary.Delay` 2.0)
  (for _array_element (`self.Weapons`)
    (if (== _array_element "/Game/Weapons/Sword/BP_Sword.BP_Sword_C")
      (`self.SwordFunction`)
      (elif (== _array_element "/Game/Weapons/Shield/BP_Shield.BP_Shield_C")
        (`self.FiringShield`)
        (elif (== _array_element "/Game/Weapons/FartAura/BP_FartAura.BP_FartAura_C")
          (`self.FireFartAura`)
          (elif (== _array_element "/Game/Weapons/MagmaFist/BP_MagmaFist.BP_MagmaFist_C")
            (`self.MagmaFistFunction`)
            (elif (== _array_element "/Game/Weapons/Chakram/BP_Chakram.BP_Chakram_C")
              (`self.ChakramFunction`)
              (elif (== _array_element "/Game/Weapons/ChainLightning/BP_ChainLightning.BP_ChainLightning_C")
                (`self.ChainLightningFunction`)))))))))

(event `self.ReceiveTick`
  (params (DeltaSeconds :type "Float (single-precision)"))
  (bind _sprite (`self.Sprite`))
  ;[1 1 1] Tick
  (if (>= (`self.Exp`) (`self.MaxExp`))
    (`self.LevelUp`))
  (if (`self.bIsDodging`)
    _
    (elif (`self.bAttacking`)
      _
      (elif (== (`self.GetVelocity`) (0.0 0.0 0.0))
        (`PaperFlipbookComponent.SetFlipbook` _sprite (`self.CharacterSprite`))
        (else
          (`PaperFlipbookComponent.SetFlipbook` _sprite (`self.CharacterMovingSprite`)))))))

(event `Key|A`
  (params (Key :type "Key Structure"))
  ;[1 1 1] Movement
  (:`Pressed`
    (set `self.Rotation` -1.0)))

(event `Key|D`
  (params (Key :type "Key Structure"))
  ;[1 1 1] Movement
  (:`Pressed`
    (set `self.Rotation` 1.0)))

(event `InputAxis|MoveRight`
  (params (AxisValue :type "Float (single-precision)"))
  ;[1 1 1] Movement
  (`self.AddMovementInput` (`KismetMathLibrary.GetForwardVector` (`KismetMathLibrary.MakeRotator` 0.0 0.0 (.yaw (`self.GetControlRotation`)))) AxisValue)
  (`SceneComponent.SetRelativeScale3D` (`self.Sprite`) (`KismetMathLibrary.MakeVector` (`self.Rotation`) 1.0 1.0)))

(event `InputAxis|MoveUp`
  (params (AxisValue :type "Float (single-precision)"))
  ;[1 1 1] Movement
  (`self.AddMovementInput` (`KismetMathLibrary.GetRightVector` (`KismetMathLibrary.MakeRotator` 0.0 0.0 (.yaw (`self.GetControlRotation`)))) AxisValue))

(event `self.ReceiveAnyDamage`
  (params (Damage :type "Float (single-precision)") (DamageType :type "DamageType Object Reference") (InstigatedBy :type "Controller Object Reference") (DamageCauser :type "Actor Object Reference"))
  ;[1 1 1] Take Damage
  (if (<= (- (`self.Health`) (- Damage (`self.Armor`))) 0.0)
    (set `self.Health` 0.0)
    (else
      (set `self.Health` (- (`self.Health`) (- Damage (`self.Armor`)))))))

(event `Key|LeftMouseButton`
  (params (Key :type "Key Structure"))
  (bind _melleattackradius (`self.MelleAttackRadius`))
  (bind _melleattackradius_2 (`self.MelleAttackRadius`))
  ;[1 1 1] BasicAttack
  (:`Pressed`
    (if (`self.bIsDodging`)
      _
      (elif (not (`self.bAttacking`))
        (set `self.bAttacking` true)
        (`PaperFlipbookComponent.SetFlipbook` (`self.Sprite`) (`self.BasicAttackSprite`))
        (if (== (`self.Rotation`) -1.0)
          (`SceneComponent.K2_AddLocalOffset` _melleattackradius (-20.0 -13.0 0.0) false true)
          (else
            (`SceneComponent.K2_AddLocalOffset` _melleattackradius (20.0 -13.0 0.0) false false)))
        (set `PrimitiveComponent.bGenerateOverlapEvents` true (`self.MelleAttackRadius`))
        ;[1 1 1] Damage Event
        (add `PrimitiveComponent.OnComponentBeginOverlap` (`self.MelleAttackRadius`) (delegate `MelleAttackOverlapEvent`))
        (`KismetSystemLibrary.Delay` 0.2)
        (set `PrimitiveComponent.bGenerateOverlapEvents` false _melleattackradius_2)
        (`SceneComponent.K2_SetRelativeLocation` _melleattackradius_2 (0.0 0.0 0.0) false false)
        (`KismetSystemLibrary.Delay` 0.8)
        (set `self.bAttacking` false)))))

(event `Key|SpaceBar`
  (params (Key :type "Key Structure"))
  ;[1 1 1] Dodge
  (:`Pressed`
    (set `self.bIsDodging` true)
    (`PaperFlipbookComponent.SetFlipbook` (`self.Sprite`) (`self.DodgdeSprite`))
    (set `self.bCanBeDamaged` false)
    (`self.LaunchCharacter` (* (`self.GetLastMovementInputVector`) (`self.DodgeLauntch`)))
    (`KismetSystemLibrary.Delay` 0.5)
    (set `self.bIsDodging` false)
    (set `self.bCanBeDamaged` true)))

(event `MelleAttackOverlapEvent`
  (params (OverlappedComponent :type "PrimitiveComponent Object Reference") (OtherActor :type "Actor Object Reference") (OtherComp :type "PrimitiveComponent Object Reference") (OtherBodyIndex :type Integer) (bFromSweep :type Boolean) (SweepResult :type "HitResult Structure (by ref)"))
  ;[1 1 1] Damage Event
  (bind _asbp_enemy (cast `/Game/Pawns2D/Enemys/BP_Enemy` OtherActor))
  (if (== (`/Game/Pawns2D/Enemys/BP_Enemy.HitBox` _asbp_enemy) OtherComp)
    (`GameplayStatics.ApplyPointDamage` _asbp_enemy (* (`self.BaseDamage`) (`self.DamageMultiplayer`)) (- (`self.K2_GetActorLocation` _asbp_enemy) (`self.K2_GetActorLocation`)) SweepResult (`self.GetController`) self "/Script/Engine.DamageType")))

(event `Key|P` :paused true
  (params (Key :type "Key Structure"))
  (:`Pressed`
    (if (`GameplayStatics.IsGamePaused`)
      (`GameplayStatics.SetGamePaused` false)
      (else
        (`GameplayStatics.SetGamePaused` true)))))

(fn `ChainLightningFunction`
  (`KismetSystemLibrary.K2_SetTimer` null "FireChainLightning" (* (`self.ChainLightningAttackSpeed`) (`self.AttackSpeedMultiplayer`)) true))

(fn `ChakramFunction`
  (`KismetSystemLibrary.K2_SetTimer` null "FireChakram" (* (`self.ChakramAttackSpeed`) (`self.AttackSpeedMultiplayer`)) true))

(fn `DrainMana`
  (`KismetSystemLibrary.K2_SetTimer` null "ShieldManaReduction" 1.0 true))

(fn `FireChainLightning`
  (if (not (< (`self.Mana`) (* (`self.ChainLightningManaCost`) (`self.ManaCostMultiplayer`))))
    (set `self.Mana` (- (`self.Mana`) (* (`self.ChainLightningManaCost`) (`self.ManaCostMultiplayer`))))
    (bind _returnvalue (`|SpawnActorFromClass` "/Game/Weapons/ChainLightning/BP_ChainLightning.BP_ChainLightning_C" (`self.GetTransform`) "AdjustIfPossibleButAlwaysSpawn" "OverrideRootScale" null self))
    (`/Game/Weapons/BP_Weapon.FireWeapon` _returnvalue)))

(fn `FireChakram`
  (if (not (< (`self.Mana`) (* (`self.ChakramManaCost`) (`self.ManaCostMultiplayer`))))
    (set `self.Mana` (- (`self.Mana`) (* (`self.ChakramManaCost`) (`self.ManaCostMultiplayer`))))
    (bind _returnvalue (`|SpawnActorFromClass` "/Game/Weapons/Chakram/BP_Chakram.BP_Chakram_C" (`self.GetTransform`) "AdjustIfPossibleButAlwaysSpawn" "OverrideRootScale" null self))
    (`/Game/Weapons/BP_Weapon.FireWeapon` _returnvalue)))

(fn `FireFartAura`
  (bind _returnvalue (`|SpawnActorFromClass` "/Game/Weapons/FartAura/BP_FartAura.BP_FartAura_C" (`self.GetTransform`) "AdjustIfPossibleButAlwaysSpawn" "OverrideRootScale" null self))
  (`/Game/Weapons/BP_Weapon.FireWeapon` _returnvalue))

(fn `FireMagmaFist`
  (bind (_returnvalue_x _returnvalue_y) (`KismetMathLibrary.BreakVector2D` (`WidgetLayoutLibrary.GetViewportSize`)))
  (if (not (< (`self.Mana`) (* (`self.MagmaFistManaCost`) (`self.ManaCostMultiplayer`))))
    (set `self.Mana` (- (`self.Mana`) (* (`self.MagmaFistManaCost`) (`self.ManaCostMultiplayer`))))
    (bind _returnvalue (`|SpawnActorFromClass` "/Game/Weapons/MagmaFist/BP_MagmaFist.BP_MagmaFist_C" (`KismetMathLibrary.MakeTransform` (`KismetMathLibrary.RandomPointInBoundingBox` (`SceneComponent.K2_GetComponentLocation` (`self.Camera`)) (`KismetMathLibrary.MakeVector` (/ _returnvalue_x 2.0) (/ _returnvalue_y 2.0) 50.0))) "AdjustIfPossibleButAlwaysSpawn" "OverrideRootScale" null self))
    (`/Game/Weapons/BP_Weapon.FireWeapon` _returnvalue)))

(fn `FireScythe`
  (bind _returnvalue (`|SpawnActorFromClass` "/Game/Weapons/Shield/BP_Shield.BP_Shield_C" (`self.GetTransform`) "AdjustIfPossibleButAlwaysSpawn" "OverrideRootScale" null self))
  (`/Game/Weapons/BP_Weapon.FireWeapon` _returnvalue))

(fn `FireSword`
  (if (not (< (`self.Mana`) (* (`self.SwordManaCost`) (`self.ManaCostMultiplayer`))))
    (set `self.Mana` (- (`self.Mana`) (* (`self.SwordManaCost`) (`self.ManaCostMultiplayer`))))
    (bind _returnvalue (`|SpawnActorFromClass` "/Game/Weapons/Sword/BP_Sword.BP_Sword_C" (`self.GetTransform`) "AdjustIfPossibleButAlwaysSpawn" "OverrideRootScale" null self))
    (`/Engine/EditorBlueprintResources/StandardMacros.IsValid` _returnvalue
      (:`Is Valid`
        (`/Game/Weapons/BP_Weapon.FireWeapon` _returnvalue)))))

(fn `FireWeapons`
  (bind _closestenemy (`self.GetClosestEnemy`))
  (`/Engine/EditorBlueprintResources/StandardMacros.IsValid` _closestenemy
    (:`Is Valid`
      (for _array_element (`self.Weapons`)
        (if (== _array_element "/Game/Weapons/Sword/BP_Sword.BP_Sword_C")
          (`KismetSystemLibrary.K2_SetTimer` null "FireSword" 1.0 true))))))

(fn `GetClosestEnemy`
  (returns (ClosestEnemy :type "/Game/Pawns2D/Enemys/BP_Enemy Object Reference"))
  (locals (CurrentlyClosestEnemy :type "/Game/Pawns2D/Enemys/BP_Enemy Object Reference"))
  (bind _outactors (`GameplayStatics.GetAllActorsOfClass` "/Game/Pawns2D/Enemys/BP_Enemy.BP_Enemy_C"))
  (set `local.CurrentlyClosestEnemy` (`|GetArrayItem` _outactors))
  (for (_array_element _array_index) _outactors
    (if (!= _array_index 0)
      (if (<= (`self.GetHorizontalDistanceTo` _array_element self) (`self.GetHorizontalDistanceTo` (`local.CurrentlyClosestEnemy`) self))
        (set `local.CurrentlyClosestEnemy` _array_element))))
  (return (`local.CurrentlyClosestEnemy`)))

(fn `HealthRegeneration`
  (if (!= (`self.Health`) (`self.MaxHealth`))
    (set `self.Health` (+ (`self.Health`) (`self.HealthRegen`))))
  (set `self.Health` (`KismetMathLibrary.FClamp` (`self.Health`) 0.0 (`self.MaxHealth`))))

(fn `LevelUp`
  (`/Engine/EditorBlueprintResources/StandardMacros.IncrementInt` (`self.Level`)
    (:`  `
      (set `self.Exp` 0.0)
      (set `self.MaxExp` (* (`self.MaxExp`) 1.2))
      (`GameplayStatics.SetGamePaused` true)
      (bind _returnvalue (`|CreateWidget` "/Game/HUD/BP_LevelUpMenu.BP_LevelUpMenu_C" (`self.PlayerControlelr`)))
      (`UserWidget.AddToViewport` _returnvalue 0)
      (`WidgetBlueprintLibrary.SetInputMode_UIOnlyEx` (`self.PlayerControlelr`) _returnvalue))))

(fn `MagmaFistFunction`
  (`KismetSystemLibrary.K2_SetTimer` null "FireMagmaFist" (* (`self.MagmaFistCooldown`) (`self.AttackSpeedMultiplayer`)) true))

(fn `ManaRegeneration`
  (if (!= (`self.Mana`) (`self.MaxMana`))
    (set `self.Mana` (+ (`self.Mana`) (`self.ManaRegen`)))
    (set `self.Mana` (`KismetMathLibrary.FClamp` (`self.Mana`) 0.0 (`self.MaxMana`)))))

(fn `ScytheFunction`
  (`KismetSystemLibrary.K2_SetTimer` null "FireScythe" 1.0 true))

(fn `ShieldManaReduction`)

(fn `SwordFunction`
  (bind _closestenemy (`self.GetClosestEnemy`))
  (`/Engine/EditorBlueprintResources/StandardMacros.IsValid` _closestenemy
    (:`Is Valid`
      (`KismetSystemLibrary.K2_SetTimer` null "FireSword" (* (`self.SwordAttackSpeed`) (`self.AttackSpeedMultiplayer`)) true))))

(fn `UserConstructionScript`)