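; BP_RangerProjectile is a homing projectile that damages enemies, using stats from the player's BP_Marko pawn.
; On BeginPlay it computes damage from base damage and multiplier, then homes on the player's closest enemy.
; Lifespan and overlap binding are set only when that target is valid.
; On overlap, it searches all BP_Enemy actors for a matching HitBox, applies point damage credited to the player, and destroys itself.
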(event `self.ReceiveBeginPlay`
  (bind _asbp_marko (cast `/Game/Pawns2D/BP_Marko` (`GameplayStatics.GetPlayerPawn` 0)))
  (bind _output_get (set `self.Player` _asbp_marko))
  (set `self.Damage` (* (`/Game/Pawns2D/BP_Marko.BaseDamage` _output_get) (`/Game/Pawns2D/BP_Marko.DamageMultiplayer` _output_get)))
  (bind _closestenemy (`/Game/Pawns2D/BP_Marko.GetClosestEnemy` (`self.Player`)))
  (`/Engine/EditorBlueprintResources/StandardMacros.IsValid` _closestenemy
    (:`Is Valid`
      (set `ProjectileMovementComponent.HomingTargetComponent` (`self.GetComponentByClass` _closestenemy "/Script/Engine.SceneComponent") (`self.ProjectileMovement`))
      (`self.SetLifeSpan` 5.0)
      (add `PrimitiveComponent.OnComponentBeginOverlap` (`self.Box`) (delegate `OnComponentBeginOverlap_Event_0`)))))

(event `OnComponentBeginOverlap_Event_0`
  (params (OverlappedComponent :type "PrimitiveComponent Object Reference") (OtherActor :type "Actor Object Reference") (OtherComp :type "PrimitiveComponent Object Reference") (OtherBodyIndex :type Integer) (bFromSweep :type Boolean) (SweepResult :type "HitResult Structure (by ref)"))
  (bind _player (`self.Player`))
  (bind _outactors (`GameplayStatics.GetAllActorsOfClass` "/Game/Pawns2D/Enemys/BP_Enemy.BP_Enemy_C"))
  (for _array_element _outactors
    (`/Engine/EditorBlueprintResources/StandardMacros.IsValid` _array_element
      (:`Is Valid`
        (if (== (`/Game/Pawns2D/Enemys/BP_Enemy.HitBox` _array_element) OtherComp)
          (`GameplayStatics.ApplyPointDamage` _array_element (`self.Damage`) (- (`self.K2_GetActorLocation` _array_element) (`self.K2_GetActorLocation`)) SweepResult (`Pawn.GetController` _player) _player "/Script/Engine.DamageType")
          (`self.K2_DestroyActor`)
          (break))))))

(fn `UserConstructionScript`)