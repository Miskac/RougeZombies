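; BP_Laser is a short-lived laser weapon actor that damages actors overlapping its box collision, ignoring the owning player.
; On BeginPlay it runs InicializeStats, which extends the parent version to set damage from the player's laser damage and damage multiplier, then sets a brief lifespan.
; The box's begin-overlap event applies that damage, crediting the player as causer and the player's controller as instigator.
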(event `self.ReceiveBeginPlay`
  (`parent.ReceiveBeginPlay`)
  (`self.InicializeStats`)
  (`self.SetLifeSpan` 0.35)
  (add `PrimitiveComponent.OnComponentBeginOverlap` (`self.Box`) (delegate `OnComponentBeginOverlap_Event_0`)))

(event `OnComponentBeginOverlap_Event_0`
  (params (OverlappedComponent :type "PrimitiveComponent Object Reference") (OtherActor :type "Actor Object Reference") (OtherComp :type "PrimitiveComponent Object Reference") (OtherBodyIndex :type Integer) (bFromSweep :type Boolean) (SweepResult :type "HitResult Structure (by ref)"))
  (bind _player (`self.Player`))
  (if (not (== (`self.Player`) OtherActor))
    (`GameplayStatics.ApplyDamage` OtherActor (`self.Damage`) (`Pawn.GetController` _player) _player "/Script/Engine.DamageType")))

(fn `InicializeStats`
  (bind _player (`self.Player`))
  (`parent.InicializeStats`)
  (set `self.Damage` (* (`/Game/Pawns2D/BP_Marko.LaserDamage` _player) (`/Game/Pawns2D/BP_Marko.DamageMultiplayer` _player))))

(fn `UserConstructionScript`
  (`parent.UserConstructionScript`))