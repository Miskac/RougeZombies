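; BP_Marko is the 2D flipbook character Marko, driven by player movement input.
; BeginPlay clamps Health and Mana to their maximums, and Tick switches the sprite between idle and run flipbooks based on velocity.
; MoveRight and MoveUp move along the control yaw's forward and right vectors respectively.
; A and D set Rotation, which MoveRight applies as the sprite's X scale to mirror its facing.
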(event `self.ReceiveBeginPlay`
  (set `self.Health` (`KismetMathLibrary.FClamp` (`self.Health`) 0.0 (`self.MaxHealth`)))
  (set `self.Mana` (`KismetMathLibrary.FClamp` (`self.Mana`) 0.0 (`self.MaxMana`))))

(event `self.ReceiveTick`
  (params (DeltaSeconds :type "Float (single-precision)"))
  (bind _sprite (`self.Sprite`))
  (if (== (`self.GetVelocity`) (0.0 0.0 0.0))
    (`PaperFlipbookComponent.SetFlipbook` _sprite "/Game/Pawns2D/Marko/WalkingSheet2/MarkoIdle2.MarkoIdle2")
    (else
      (`PaperFlipbookComponent.SetFlipbook` _sprite "/Game/Pawns2D/Marko/WalkingSheet2/MarkoRun2.MarkoRun2"))))

(event `Key|A`
  (params (Key :type "Key Structure"))
  (:`Pressed`
    (set `self.Rotation` -1.0)))

(event `Key|D`
  (params (Key :type "Key Structure"))
  (:`Pressed`
    (set `self.Rotation` 1.0)))

(event `InputAxis|MoveRight`
  (params (AxisValue :type "Float (single-precision)"))
  (`self.AddMovementInput` (`KismetMathLibrary.GetForwardVector` (`KismetMathLibrary.MakeRotator` 0.0 0.0 (.yaw (`self.GetControlRotation`)))) AxisValue)
  (`SceneComponent.SetRelativeScale3D` (`self.Sprite`) (`KismetMathLibrary.MakeVector` (`self.Rotation`) 1.0 1.0)))

(event `InputAxis|MoveUp`
  (params (AxisValue :type "Float (single-precision)"))
  (`self.AddMovementInput` (`KismetMathLibrary.GetRightVector` (`KismetMathLibrary.MakeRotator` 0.0 0.0 (.yaw (`self.GetControlRotation`)))) AxisValue))

(fn `UserConstructionScript`)