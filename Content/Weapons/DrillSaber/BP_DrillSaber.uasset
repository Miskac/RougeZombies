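; BP_DrillSaber is a projectile weapon that launches toward the closest enemy and damages enemies it passes through.
; On spawn it aims horizontally at that enemy and sets a three-second lifespan, both only if a target exists.
; InicializeStats scales damage from the player's DrillSaber stat and multiplier.
; Each HitBox overlap searches all BP_Enemy actors for a matching hitbox before applying player-credited damage, without destroying the projectile.
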(event `self.ReceiveBeginPlay`
  (bind _projectilemovement (`self.ProjectileMovement`))
  (`parent.ReceiveBeginPlay`)
  (`self.InicializeStats`)
  (add `PrimitiveComponent.OnComponentBeginOverlap` (`self.HitBox`) (delegate `OnComponentBeginOverlap_Event_0`))
  (bind _closesenemy (`self.GetClosestEnemy`))
  (`/Engine/EditorBlueprintResources/StandardMacros.IsValid` _closesenemy
    (:`Is Valid`
      (set `MovementComponent.Velocity` (* (`ProjectileMovementComponent.InitialSpeed` _projectilemovement) (`KismetMathLibrary.Vector_Normal2D` (- (`self.K2_GetActorLocation` _closesenemy) (`self.K2_GetActorLocation`)))) _projectilemovement)
      (`self.SetLifeSpan` 3.0))))

(event `OnComponentBeginOverlap_Event_0`
  (params (OverlappedComponent :type "PrimitiveComponent Object Reference") (OtherActor :type "Actor Object Reference") (OtherComp :type "PrimitiveComponent Object Reference") (OtherBodyIndex :type Integer) (bFromSweep :type Boolean) (SweepResult :type "HitResult Structure (by ref)"))
  (bind _player (`self.Player`))
  (bind _outactors (`GameplayStatics.GetAllActorsOfClass` "/Game/Pawns2D/Enemys/BP_Enemy.BP_Enemy_C"))
  (for _array_element _outactors
    (`/Engine/EditorBlueprintResources/StandardMacros.IsValid` _array_element
      (:`Is Valid`
        (if (== (`/Game/Pawns2D/Enemys/BP_Enemy.HitBox` _array_element) OtherComp)
          (`GameplayStatics.ApplyDamage` OtherActor (`self.Damage`) (`Pawn.GetController` _player) _player "/Script/Engine.DamageType"))))))

(fn `InicializeStats`
  (bind _player (`self.Player`))
  (`parent.InicializeStats`)
  (set `self.Damage` (* (`/Game/Pawns2D/BP_Marko.DrillSaberDamage` _player) (`/Game/Pawns2D/BP_Marko.DamageMultiplayer` _player))))

(fn `UserConstructionScript`
  (`parent.UserConstructionScript`))