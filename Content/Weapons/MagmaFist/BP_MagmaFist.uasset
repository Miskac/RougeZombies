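; Magma Fist player weapon: a homing projectile that turns into a damaging lava pool when it hits an enemy.
; FireWeapon homes it on the closest enemy, and its stats and lifespan come from the Player's MagmaFist values and multipliers.
; On enemy HitBox overlap it stops, swaps to the LavaPool flipbook, rescales and snaps to a fixed height.
; A looping timer then damages every overlapping enemy; the mana deduction in DealDamage is disconnected.
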(event `self.ReceiveBeginPlay`
  (`parent.ReceiveBeginPlay`)
  (`self.InicializeStats`)
  (`self.SetLifeSpan` (`self.MagmaDuration`))
  (add `PrimitiveComponent.OnComponentBeginOverlap` (`self.HitBox`) (delegate `OnComponentBeginOverlap_Event_0`)))

(event `OnComponentBeginOverlap_Event_0`
  (params (OverlappedComponent :type "PrimitiveComponent Object Reference") (OtherActor :type "Actor Object Reference") (OtherComp :type "PrimitiveComponent Object Reference") (OtherBodyIndex :type Integer) (bFromSweep :type Boolean) (SweepResult :type "HitResult Structure (by ref)"))
  (bind _hitbox (`self.HitBox`))
  (bind _weaponsprite (`self.WeaponSprite`))
  (bind (_returnvalue_x _returnvalue_y) (`KismetMathLibrary.BreakVector` (`SceneComponent.K2_GetComponentLocation` _hitbox)))
  (bind (_returnvalue_x_2 _returnvalue_y_2) (`KismetMathLibrary.BreakVector` (`SceneComponent.K2_GetComponentLocation` _weaponsprite)))
  (bind _outactors (`GameplayStatics.GetAllActorsOfClass` "/Game/Pawns2D/Enemys/BP_Enemy.BP_Enemy_C"))
  (for _array_element _outactors
    (if (== (`/Game/Pawns2D/Enemys/BP_Enemy.HitBox` _array_element) OtherComp)
      (`PaperFlipbookComponent.SetFlipbook` (`self.WeaponSprite`) "/Game/Weapons/MagmaFist/Sprite/LavaPool.LavaPool")
      (set `ProjectileMovementComponent.bIsHomingProjectile` false (`self.ProjectileMovement`))
      (`MovementComponent.StopMovementImmediately` (`self.ProjectileMovement`))
      (`SceneComponent.SetRelativeScale3D` (`self.WeaponSprite`) (* (`self.BaseSizeScale`) (`self.SizeScale`)))
      (`SceneComponent.SetRelativeScale3D` (`self.HitBox`) (`self.SizeScale`))
      (`SceneComponent.K2_SetWorldLocation` _hitbox (`KismetMathLibrary.MakeVector` _returnvalue_x _returnvalue_y 40.0) false true)
      (`SceneComponent.K2_SetWorldLocation` _weaponsprite (`KismetMathLibrary.MakeVector` _returnvalue_x_2 _returnvalue_y_2 40.0) false true)
      (`KismetSystemLibrary.K2_SetTimer` null "DealDamage" (`self.AttackSpeed`) true))))

(fn `DealDamage`
  (bind _player (`self.Player`))
  (for _array_element (`PrimitiveComponent.GetOverlappingActors` (`self.HitBox`) "/Game/Pawns2D/Enemys/BP_Enemy.BP_Enemy_C")
    (`GameplayStatics.ApplyDamage` _array_element (`self.Damage`) (`Pawn.GetController` _player) _player "/Script/Engine.DamageType")))

(fn `FireWeapon`
  (`parent.FireWeapon`)
  (bind _closesenemy (`self.GetClosestEnemy`))
  (set `ProjectileMovementComponent.HomingTargetComponent` (`self.GetComponentByClass` _closesenemy "/Script/Engine.SceneComponent") (`self.ProjectileMovement`)))

(fn `InicializeStats`
  (bind _player (`self.Player`))
  (`parent.InicializeStats`)
  (set `self.Damage` (* (`/Game/Pawns2D/BP_Marko.MagmaFistDamage` _player) (`/Game/Pawns2D/BP_Marko.DamageMultiplayer` _player)))
  (set `self.ManaCost` (* (`/Game/Pawns2D/BP_Marko.MagmaFistManaCost` _player) (`/Game/Pawns2D/BP_Marko.ManaCostMultiplayer` _player)))
  (set `self.AttackSpeed` (* (`/Game/Pawns2D/BP_Marko.MagmaFistAttackSpeed` _player) (`/Game/Pawns2D/BP_Marko.AttackSpeedMultiplayer` _player)))
  (set `self.MagmaDuration` (`/Game/Pawns2D/BP_Marko.MagmaFistDuration` _player))
  (set `self.SizeScale` (`/Game/Pawns2D/BP_Marko.MagmaFistSizeScale` _player)))

(fn `UserConstructionScript`
  (`parent.UserConstructionScript`))