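; Blue Witch projectile that deals point damage to enemies on behalf of the BP_Marko player pawn.
; On spawn it computes damage from the player's base damage and multiplier, and sets a short lifespan.
; Its velocity uses the 2D-normalized end point of the cursor trace, without subtracting the projectile's location.
; HitBox overlaps are matched against every BP_Enemy's HitBox, damaging the match and destroying the projectile.
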(event `self.ReceiveBeginPlay`
  (bind _asbp_marko (cast `/Game/Pawns2D/BP_Marko` (`GameplayStatics.GetPlayerPawn` 0)))
  (bind _output_get (set `self.Player` _asbp_marko))
  (set `self.Damage` (* (`/Game/Pawns2D/BP_Marko.BaseDamage` _output_get) (`/Game/Pawns2D/BP_Marko.DamageMultiplayer` _output_get)))
  (bind _asbp_player_controller (cast `/Game/Controller/BP_PlayerController` (`Pawn.GetController` (`self.Player`))))
  (set `MovementComponent.Velocity` (* (`KismetMathLibrary.Vector_Normal2D` (`.TraceEnd` (`GameplayStatics.BreakHitResult` (`PlayerController.GetHitResultUnderCursorByChannel` _asbp_player_controller "TraceTypeQuery2" false)))) (`ProjectileMovementComponent.InitialSpeed` (`self.ProjectileMovement`))) (`self.ProjectileMovement`))
  (add `PrimitiveComponent.OnComponentBeginOverlap` (`self.HitBox`) (delegate `OnComponentBeginOverlap_Event_0`))
  (`self.SetLifeSpan` 4.0))

(event `OnComponentBeginOverlap_Event_0`
  (params (OverlappedComponent :type "PrimitiveComponent Object Reference") (OtherActor :type "Actor Object Reference") (OtherComp :type "PrimitiveComponent Object Reference") (OtherBodyIndex :type Integer) (bFromSweep :type Boolean) (SweepResult :type "HitResult Structure (by ref)"))
  (bind _player (`self.Player`))
  (bind _outactors (`GameplayStatics.GetAllActorsOfClass` "/Game/Pawns2D/Enemys/BP_Enemy.BP_Enemy_C"))
  (for _array_element _outactors
    (`/Engine/EditorBlueprintResources/StandardMacros.IsValid` _array_element
      (:`Is Valid`
        (if (== (`/Game/Pawns2D/Enemys/BP_Enemy.HitBox` _array_element) OtherComp)
          (`GameplayStatics.ApplyPointDamage` _array_element (`self.Damage`) (- (`self.K2_GetActorLocation` _array_element) (`self.K2_GetActorLocation`)) SweepResult (`Pawn.GetController` _player) _player "/Script/Engine.DamageType")
          (`self.K2_DestroyActor`)
          (break))))))

(fn `UserConstructionScript`)