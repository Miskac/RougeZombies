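; BP_Shield is a scythe weapon actor that orbits the player and damages enemies it touches.
; Tick rotates an offset around the player at a speed set by scythe attack speed, using stats copied from the player.
; HitBox overlaps deal point damage reduced by enemy armor, then briefly disable overlaps.
; A one-second looping timer drains mana, switching overlaps off when mana is insufficient.
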(event `self.ReceiveBeginPlay`
  (`parent.ReceiveBeginPlay`)
  (`self.InicializeStats`)
  (`KismetSystemLibrary.K2_SetTimer` null "DrainMana" 1.0 true)
  ;[1 1 1] Damage event
  (add `PrimitiveComponent.OnComponentBeginOverlap` (`self.HitBox`) (delegate `OnComponentBeginOverlap_Event_0`)))

(event `OnComponentBeginOverlap_Event_0`
  (params (OverlappedComponent :type "PrimitiveComponent Object Reference") (OtherActor :type "Actor Object Reference") (OtherComp :type "PrimitiveComponent Object Reference") (OtherBodyIndex :type Integer) (bFromSweep :type Boolean) (SweepResult :type "HitResult Structure (by ref)"))
  (bind _player (`self.Player`))
  ;[1 1 1] Damage event
  (bind _outactors (`GameplayStatics.GetAllActorsOfClass` "/Game/Pawns2D/Enemys/BP_Enemy.BP_Enemy_C"))
  (for _array_element _outactors
    (`/Engine/EditorBlueprintResources/StandardMacros.IsValid` _array_element
      (:`Is Valid`
        (if (and (== (`/Game/Pawns2D/Enemys/BP_Enemy.HitBox` _array_element) OtherComp) (== OtherActor _array_element))
          (`GameplayStatics.ApplyPointDamage` _array_element (- (`self.Damage`) (`/Game/Pawns2D/Enemys/BP_Enemy.Armor` _array_element)) (- (`self.K2_GetActorLocation` _array_element) (`self.K2_GetActorLocation`)) SweepResult (`Pawn.GetController` _player) _player "/Script/Engine.DamageType")
          (set `PrimitiveComponent.bGenerateOverlapEvents` false (`self.HitBox`))
          (`KismetSystemLibrary.Delay` 0.1)
          (set `PrimitiveComponent.bGenerateOverlapEvents` true (`self.HitBox`)))))))

(event `self.ReceiveTick`
  (params (DeltaSeconds :type "Float (single-precision)"))
  (`parent.ReceiveTick` DeltaSeconds)
  (set `self.NewLocation` (`self.K2_GetActorLocation` (`self.Player`)))
  (set `self.AngleAxis` (- (`self.AngleAxis`) (* DeltaSeconds (`self.Multiplayer`))))
  (if (<= (`self.AngleAxis`) -360.0)
    (set `self.AngleAxis` 0.0))
  (set `self.RotateValue` (`KismetMathLibrary.RotateAngleAxis` (`self.Dimentions`) (`self.AngleAxis`) (`self.AxisVector`)))
  (set `self.NewLocation` (+ (`self.NewLocation`) (`self.RotateValue`)))
  (bind _output_get (set `self.NewRotation` (`KismetMathLibrary.MakeRotator` 0.0 0.0 (`self.AngleAxis`))))
  (set `self.QuatRotation` (`KismetMathLibrary.Conv_RotatorToQuaternion` _output_get))
  (`self.K2_SetActorLocationAndRotation` (`self.NewLocation`) (`KismetMathLibrary.Quat_Rotator` (`self.QuatRotation`))))

(fn `DrainMana`
  (bind _player (`self.Player`))
  (if (< (`/Game/Pawns2D/BP_Marko.Mana` (`self.Player`)) (`self.ManaCost`))
    (set `PrimitiveComponent.bGenerateOverlapEvents` false (`self.HitBox`))
    (else
      (set `/Game/Pawns2D/BP_Marko.Mana` (- (`/Game/Pawns2D/BP_Marko.Mana` _player) (`self.ManaCost`)) _player)
      (set `PrimitiveComponent.bGenerateOverlapEvents` true (`self.HitBox`)))))

(fn `FireWeapon`
  (`parent.FireWeapon`))

(fn `InicializeStats`
  (bind _player (`self.Player`))
  (`parent.InicializeStats`)
  (set `self.Damage` (* (`/Game/Pawns2D/BP_Marko.ScytheDamage` _player) (`/Game/Pawns2D/BP_Marko.BaseDamageAmplifier` _player)))
  (set `self.ManaCost` (`/Game/Pawns2D/BP_Marko.ScytheManaCost` _player))
  (set `self.NumberOfProjectiles` (`/Game/Pawns2D/BP_Marko.NumberOfScytheProjectiles` _player))
  (set `self.Multiplayer` (`/Game/Pawns2D/BP_Marko.ScytheAttackSpeed` _player)))

(fn `UserConstructionScript`
  (`parent.UserConstructionScript`))