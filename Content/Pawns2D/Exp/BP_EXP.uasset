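; BP_EXP is an experience pickup pawn that travels to the player and grants experience on arrival.
; On BeginPlay it caches the game mode and the BP_Marko player, then binds its Pickup component's overlap event.
; Overlapping the player's PickupRadius starts an AI MoveTo that targets the player.
; When the move succeeds, it adds ExpAmount to the player's Exp and destroys itself.
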(event `self.ReceiveBeginPlay`
  (bind _asbp_game_mode (cast `/Game/GameMode/BP_GameMode` (`GameplayStatics.GetGameMode`)))
  (set `self.GameMode` _asbp_game_mode)
  (bind _asbp_marko (cast `/Game/Pawns2D/BP_Marko` (`GameplayStatics.GetPlayerPawn` 0)))
  (set `self.Player` _asbp_marko)
  (add `PrimitiveComponent.OnComponentBeginOverlap` (`self.Pickup`) (delegate `OnComponentBeginOverlap_Event_0`)))

(event `OnComponentBeginOverlap_Event_0`
  (params (OverlappedComponent :type "PrimitiveComponent Object Reference") (OtherActor :type "Actor Object Reference") (OtherComp :type "PrimitiveComponent Object Reference") (OtherBodyIndex :type Integer) (bFromSweep :type Boolean) (SweepResult :type "HitResult Structure (by ref)"))
  (bind _player (`self.Player`))
  (bind _player_2 (`self.Player`))
  (if (== (`/Game/Pawns2D/BP_Marko.PickupRadius` (`self.Player`)) OtherComp)
    (`|AIMoveTo` self (`self.K2_GetActorLocation` _player_2) _player_2 0.0
      (:`OnSuccess`
        (set `/Game/Pawns2D/BP_Marko.Exp` (+ (`/Game/Pawns2D/BP_Marko.Exp` _player) (`self.ExpAmount`)) _player)
        (`self.K2_DestroyActor`)))))

(fn `UserConstructionScript`)