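; Bombino weapon projectile that homes in on the closest enemy found at spawn and explodes on contact, expiring after a short lifespan.
; Damage comes from the Player's Bombino damage and multiplier.
; A HitBox overlap with any BP_Enemy plays the explosion flipbook, applies radial falloff damage that ignores the Player, then destroys the actor after a brief delay.
; Tick mirrors the sprite to match horizontal travel direction.
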(event `self.ReceiveBeginPlay`
  (`parent.ReceiveBeginPlay`)
  (`self.InicializeStats`)
  (bind _closesenemy (`self.GetClosestEnemy`))
  (set `ProjectileMovementComponent.HomingTargetComponent` (`self.GetComponentByClass` _closesenemy "/Script/Engine.SceneComponent") (`self.ProjectileMovement`))
  (add `PrimitiveComponent.OnComponentBeginOverlap` (`self.HitBox`) (delegate `OnComponentBeginOverlap_Event_0`))
  (`self.SetLifeSpan` 5.0))

(event `OnComponentBeginOverlap_Event_0`
  (params (OverlappedComponent :type "PrimitiveComponent Object Reference") (OtherActor :type "Actor Object Reference") (OtherComp :type "PrimitiveComponent Object Reference") (OtherBodyIndex :type Integer) (bFromSweep :type Boolean) (SweepResult :type "HitResult Structure (by ref)"))
  (bind _player (`self.Player`))
  (bind _outactors (`GameplayStatics.GetAllActorsOfClass` "/Game/Pawns2D/Enemys/BP_Enemy.BP_Enemy_C"))
  (for _array_element _outactors
    (`/Engine/EditorBlueprintResources/StandardMacros.IsValid` _array_element
      (:`Is Valid`
        (if (== _array_element OtherActor)
          (`PaperFlipbookComponent.SetFlipbook` (`self.WeaponSprite`) "/Game/Weapons/Bombino/Sprite/BombinoExplode.BombinoExplode")
          (`GameplayStatics.ApplyRadialDamageWithFalloff` (`self.Damage`) 5.0 (`self.K2_GetActorLocation`) 25.0 70.0 1.0 "/Script/Engine.DamageType" (`|MakeArray` _player :!type "Actor Object Reference") _player (`Pawn.GetController` _player))
          (`KismetSystemLibrary.Delay` 0.2)
          (`self.K2_DestroyActor`)
          (break))))))

(event `self.ReceiveTick`
  (params (DeltaSeconds :type "Float (single-precision)"))
  (bind _returnvalue_x (`KismetMathLibrary.BreakVector` (`self.K2_GetActorLocation`)))
  (bind _returnvalue_x_2 (`KismetMathLibrary.BreakVector` (`self.K2_GetActorLocation`)))
  (`parent.ReceiveTick` DeltaSeconds)
  (if (> (`self.OldX`) _returnvalue_x)
    (`SceneComponent.SetRelativeScale3D` (`self.WeaponSprite`) (-1.0 1.0 1.0))
    (else
      (`SceneComponent.SetRelativeScale3D` (`self.WeaponSprite`) (1.0 1.0 1.0))))
  (set `self.OldX` _returnvalue_x_2))

(fn `InicializeStats`
  (bind _player (`self.Player`))
  (`parent.InicializeStats`)
  (set `self.Damage` (* (`/Game/Pawns2D/BP_Marko.BombinoDamage` _player) (`/Game/Pawns2D/BP_Marko.DamageMultiplayer` _player))))

(fn `UserConstructionScript`
  (`parent.UserConstructionScript`))