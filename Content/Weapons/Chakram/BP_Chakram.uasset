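; Chakram weapon projectile that damages enemies and bounces off them, extending a parent weapon class.
; FireWeapon launches it in a random horizontal direction at the projectile component's initial speed.
; HitBox overlaps are matched against every enemy's hitbox, applying point damage scaled by the player's amplifier minus enemy armor.
; Each hit reverses horizontal velocity and zeroes vertical, until the bounce limit or short lifespan destroys it.
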(event `self.ReceiveBeginPlay`
  (`parent.ReceiveBeginPlay`)
  (set `self.Damage` 10.0)
  (set `self.ManaCost` 1.0)
  (add `PrimitiveComponent.OnComponentBeginOverlap` (`self.HitBox`) (delegate `OnComponentBeginOverlap_Event_0`))
  (`self.SetLifeSpan` 5.0))

(event `OnComponentBeginOverlap_Event_0`
  (params (OverlappedComponent :type "PrimitiveComponent Object Reference") (OtherActor :type "Actor Object Reference") (OtherComp :type "PrimitiveComponent Object Reference") (OtherBodyIndex :type Integer) (bFromSweep :type Boolean) (SweepResult :type "HitResult Structure (by ref)"))
  (bind _player (`self.Player`))
  (bind _projectilemovement (`self.ProjectileMovement`))
  (bind _outactors (`GameplayStatics.GetAllActorsOfClass` "/Game/Pawns2D/Enemys/BP_Enemy.BP_Enemy_C"))
  (for _array_element _outactors
    (if (== (`/Game/Pawns2D/Enemys/BP_Enemy.HitBox` _array_element) OtherComp)
      (`/Engine/EditorBlueprintResources/StandardMacros.IncrementInt` (`self.Bounces`)
        (:`  `
          (`GameplayStatics.ApplyPointDamage` _array_element (- (* (`self.Damage`) (`/Game/Pawns2D/BP_Marko.BaseDamageAmplifier` (`self.Player`))) (`/Game/Pawns2D/Enemys/BP_Enemy.Armor` _array_element)) (`self.K2_GetActorLocation`) SweepResult (`Pawn.GetController` _player) _player "/Script/Engine.DamageType")
          (if (>= (`self.Bounces`) (`self.MaxBounces`))
            (`self.K2_DestroyActor`)
            (break)
            (else
              (set `MovementComponent.Velocity` (* (`MovementComponent.Velocity` _projectilemovement) (-1.0 -1.0 0.0)) _projectilemovement)
              (break))))))))

(fn `FireWeapon`
  (bind _projectilemovement (`self.ProjectileMovement`))
  (`parent.FireWeapon`)
  (set `MovementComponent.Velocity` (* (`KismetMathLibrary.Vector_Normal2D` (`KismetMathLibrary.RandomUnitVector`)) (`ProjectileMovementComponent.InitialSpeed` _projectilemovement)) _projectilemovement))

(fn `UserConstructionScript`
  (`parent.UserConstructionScript`))