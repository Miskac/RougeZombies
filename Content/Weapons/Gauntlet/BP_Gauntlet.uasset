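; BP_Gauntlet is a short-lived gauntlet projectile weapon that deals scaled player damage to enemies.
; On BeginPlay it fires along the X axis in a direction chosen from the player's rotation, flipping its root when reversed, and expires after a few seconds.
; Damage comes from the player's gauntlet damage and multiplier.
; HitBox overlaps are matched against all BP_Enemy actors, applying point damage and destroying the projectile.
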(event `self.ReceiveBeginPlay`
  (bind _projectilemovement (`self.ProjectileMovement`))
  (bind _projectilemovement_2 (`self.ProjectileMovement`))
  (`parent.ReceiveBeginPlay`)
  (`self.InicializeStats`)
  (`self.SetLifeSpan` 3.0)
  (if (> (`/Game/Pawns2D/BP_Marko.Rotation` (`self.Player`)) 0.0)
    (set `MovementComponent.Velocity` (`KismetMathLibrary.MakeVector` (`ProjectileMovementComponent.InitialSpeed` _projectilemovement_2)) _projectilemovement_2)
    (else
      (set `MovementComponent.Velocity` (`KismetMathLibrary.MakeVector` (* (`ProjectileMovementComponent.InitialSpeed` _projectilemovement) -1.0)) _projectilemovement)
      (`SceneComponent.K2_SetWorldRotation` (`self.DefaultSceneRoot`) (`KismetMathLibrary.MakeRotator` 180.0 0.0 180.0) false false)))
  (add `PrimitiveComponent.OnComponentBeginOverlap` (`self.HitBox`) (delegate `OnComponentBeginOverlap_Event_0`)))

(event `OnComponentBeginOverlap_Event_0`
  (params (OverlappedComponent :type "PrimitiveComponent Object Reference") (OtherActor :type "Actor Object Reference") (OtherComp :type "PrimitiveComponent Object Reference") (OtherBodyIndex :type Integer) (bFromSweep :type Boolean) (SweepResult :type "HitResult Structure (by ref)"))
  (bind _player (`self.Player`))
  (bind _outactors (`GameplayStatics.GetAllActorsOfClass` "/Game/Pawns2D/Enemys/BP_Enemy.BP_Enemy_C"))
  (for _array_element _outactors
    (`/Engine/EditorBlueprintResources/StandardMacros.IsValid` _array_element
      (:`Is Valid`
        (if (== _array_element OtherActor)
          (`GameplayStatics.ApplyPointDamage` OtherActor (`self.Damage`) (- (`self.K2_GetActorLocation` OtherActor) (`self.K2_GetActorLocation`)) SweepResult (`Pawn.GetController` _player) _player "/Script/Engine.DamageType")
          (`self.K2_DestroyActor`)
          (break))))))

(fn `InicializeStats`
  (bind _player (`self.Player`))
  (`parent.InicializeStats`)
  (set `self.Damage` (* (`/Game/Pawns2D/BP_Marko.GauntletDamage` _player) (`/Game/Pawns2D/BP_Marko.DamageMultiplayer` _player))))

(fn `UserConstructionScript`
  (`parent.UserConstructionScript`))