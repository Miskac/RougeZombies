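; BP_HammerExplosion is a short-lived explosion actor for the hammer weapon that deals area damage around its spawn location.
; On BeginPlay it runs InicializeStats, which extends the parent version by setting Damage from the Player's hammer explosion damage and damage multiplier.
; It then sets a half-second lifespan and applies one full-damage radial hit in a small radius, ignoring the Player and crediting them as causer and instigator.
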(event `self.ReceiveBeginPlay`
  (bind _player (`self.Player`))
  (`parent.ReceiveBeginPlay`)
  (`self.InicializeStats`)
  (`self.SetLifeSpan` 0.5)
  (`GameplayStatics.ApplyRadialDamage` (`self.Damage`) (`self.K2_GetActorLocation`) 60.0 "/Script/Engine.DamageType" (`|MakeArray` _player :!type "Actor Object Reference") _player (`Pawn.GetController` _player) true))

(fn `InicializeStats`
  (bind _player (`self.Player`))
  (`parent.InicializeStats`)
  (set `self.Damage` (* (`/Game/Pawns2D/BP_Marko.HammerExplosionDamage` _player) (`/Game/Pawns2D/BP_Marko.DamageMultiplayer` _player))))

(fn `UserConstructionScript`
  (`parent.UserConstructionScript`))